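; Grid manager actor that generates a tile grid centred on its own location, triggered by an editor-called event.
; It snaps the centre to tile size, derives the bottom-left corner with even/odd correction, then registers each X/Y index in TileDataLibrary.
; With VisualiseDebug on, tiles render as instanced meshes, raised against Z-fighting and tracked by a parallel ID array.
; Helpers convert indices to locations and configure the grid mesh's appearance and collision.
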(event Custom|GenerateGrid
  ;[1 1 1] Editor called function that clears the grid and then generates a new grid
  (CallFunction|ClearGrid)
  (CallFunction|IterateTiles (Transformation|GetActorLocation) (Variables|Default|GetGrid_TileSize) (Variables|Default|GetGrid_Dimensions)))

(fn ConstructionScript)

(fn IterateTiles
  (params (Centre_Location :type Vector) (TileSize :type Vector) (Dimensions :type Int%20Point%20Structure) (Tile_Data :type ST%20Tile%20Data%20Structure))
  ;[1 1 1] Saves variables for later use throughout grid lifespan
  (Variables|Default|SetGrid_Centre_Location Centre_Location)
  (Variables|Default|SetGrid_TileSize TileSize)
  (Variables|Default|SetGrid_Dimensions Dimensions)
  ;[1 1 1] Apply grid offset to stop Z-Fighting
  (Transformation|SetWorldLocation (Variables|Default|GetInstancedGridMesh) (Math|Vector|MakeVector 0.0 0.0 (Variables|Default|GetGrid_Offset_From_Ground)) false false)
  ;[1 1 1] Calculates the grid centre offset so the grid is always centred on the gridmanager actor transform
  (bind (_centre _bottomleft) (CallFunction|CalculateGridCentre&BottomLeft))
  (Variables|Default|SetGrid_Centre_Location _centre)
  (Variables|Default|SetGrid_BottomLeft_Location _bottomleft)
  ;[1 1 1] Iterates through the X & Y positions of our grid to update each tile's state. Then saves the current tile's X & Y coordinate for storingg in the Index
  (for _index (range 0 (- (.x (Variables|Default|GetGrid_Dimensions)) 1))
    (LocalVariables|SetX _index)
    (for _index_2 (range 0 (- (.y (Variables|Default|GetGrid_Dimensions)) 1))
      (LocalVariables|SetY _index_2)
      ;[1 1 1] Tile ID (This tracks our current progress and selected tile.)
      (bind _output_get (LocalVariables|SetCurrent%20Tile%20ID (Utilities|Struct|MakeIntPoint (LocalVariables|GetX) (LocalVariables|GetY))))
      (Utilities|Map|Add :TargetMap (Variables|Default|GetTile_Data_Library) :Key _output_get)
      (bind _output_get_2 (Variables|Default|SetCurrentTileTransform (Math|Transform|MakeTransform (CallFunction|GetTileLocationfromGridIndex (LocalVariables|GetCurrent%20Tile%20ID)) "0, 0, 0" "1.000000,1.000000,1.000000")))
      (if (Variables|Default|GetVisualiseDebug)
        (CallFunction|AddTileInstance _output_get_2 _output_get)))))

(fn ClearGrid
  ;[1 1 1] Clears all of the mesh instances from the grid and then clears the Tile ID Array
  (Components|InstancedStaticMesh|ClearInstances (Variables|Default|GetInstancedGridMesh))
  (Utilities|Array|Clear (Variables|Default|GetInstanceIDs)))

(fn CalculateGridCentre&BottomLeft
  (bind _grid_dimensions (Variables|Default|GetGrid_Dimensions))
  (LocalVariables|SetC (CallFunction|SnapVectortoVector (Variables|Default|GetGrid_Centre_Location) (Variables|Default|GetGrid_TileSize)))
  (return (LocalVariables|GetC) (- (LocalVariables|GetC) (* (/ (- (Variables|Default|GetGrid_Dimensions) (Math|Vector2D|MakeVector2D (Math|Float|SelectFloat 0.0 1.0 (CallFunction|IsIntEven? (.x _grid_dimensions))) (Math|Float|SelectFloat 0.0 1.0 (CallFunction|IsIntEven? (.y _grid_dimensions))))) 2.0) (Variables|Default|GetGrid_TileSize)))))

(fn GetTileLocationfromGridIndex
  (params (GridIndex :type Int%20Point%20Structure))
  (return (+ (Variables|Default|GetGrid_BottomLeft_Location) (* (Variables|Default|GetGrid_TileSize) (Math|Conversions|ToVector2D(IntPoint) GridIndex)))))

(fn GetTileRotationfromGridIndex
  (params (Grid%20Index :type Int%20Point%20Structure))
  (return "0, 0, 0"))

(fn AddTileInstance
  (params (Transform :type Transform) (ID :type Int%20Point%20Structure%20%28by%20ref%29))
  (CallFunction|RemoveInstance ID)
  (Components|InstancedStaticMesh|AddInstance (Variables|Default|GetInstancedGridMesh) Transform false)
  (Utilities|Array|Add (Variables|Default|GetInstanceIDs) ID))

(fn RemoveInstance
  (params (ID%20To%20Remove :type Int%20Point%20Structure%20%28by%20ref%29))
  (bind _instanceids (Variables|Default|GetInstanceIDs))
  (if (Utilities|Array|ContainsItem _instanceids ID%20To%20Remove)
    (Class|InstancedStaticMeshComponent|RemoveInstance (Variables|Default|GetInstancedGridMesh) (Utilities|Array|FindItem _instanceids ID%20To%20Remove))
    (Utilities|Array|RemoveItem (Variables|Default|GetInstanceIDs) ID%20To%20Remove)))

(fn InitializeGridMeshVisual
  (params (Mesh :type Static%20Mesh%20Object%20Reference) (Material :type Material%20Interface%20Object%20Reference) (Colour :type Linear%20Color%20Structure) (Collision :type ECollisionEnabled%20Enum :default "NoCollision"))
  (Components|StaticMesh|SetStaticMesh (Variables|Default|GetInstancedGridMesh) Mesh)
  (Rendering|Material|SetMaterial (Variables|Default|GetInstancedGridMesh) 0 Material)
  (Rendering|Material|SetVectorParameterValueonMaterials (Variables|Default|GetInstancedGridMesh) "Colour" (Math|Conversions|ToVector(LinearColor) Colour))
  (Collision|SetCollisionEnabled (Variables|Default|GetInstancedGridMesh) Collision))