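; BP_GridDebugPawn is a camera pawn in the grid system's debug tools, providing pan, zoom and stepped rotation.
; Enhanced Input actions adjust desired location, spring-arm length and rotation, with zoom clamped to limits and yaw stepped once per press.
; Tick interpolates the actor transform and spring-arm length toward those targets, smoothing motion without sweeping for collision.
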(event Input|EnhancedActionEvents|EnhancedInputActionGIA_Zoom
  (params (ActionValue :type Float%20%28double-precision%29) (ElapsedSeconds :type Float%20%28double-precision%29) (TriggeredSeconds :type Float%20%28double-precision%29) (InputAction :type Input%20Action%20Object%20Reference :default "/Game/Systems/GridSystem/DebugTools/DebugInputs/InputActions/GIA_Zoom.GIA_Zoom"))
  ;[1 1 1] Zoom logic
  (:Triggered
    (Variables|Default|SetZoom_Desired (Math|Float|Clamp(Float) (+ (* ActionValue (Variables|Default|GetZoom_Speed)) (Variables|Default|GetZoom_Desired)) (Variables|Default|GetZoom_Min) (Variables|Default|GetZoom_Max)))))

(event Input|EnhancedActionEvents|EnhancedInputActionGIA_Forwards
  (params (ActionValue :type Float%20%28double-precision%29) (ElapsedSeconds :type Float%20%28double-precision%29) (TriggeredSeconds :type Float%20%28double-precision%29) (InputAction :type Input%20Action%20Object%20Reference :default "/Game/Systems/GridSystem/DebugTools/DebugInputs/InputActions/GIA_Forwards.GIA_Forwards"))
  ;[1 1 1] Movement Logic
  (:Triggered
    (Variables|Default|SetLocation_Desired (+ (* (* ActionValue (Variables|Default|GetLocation_Speed)) (Transformation|GetActorForwardVector)) (Variables|Default|GetLocation_Desired)))))

(event Input|EnhancedActionEvents|EnhancedInputActionGIA_Sideways
  (params (ActionValue :type Float%20%28double-precision%29) (ElapsedSeconds :type Float%20%28double-precision%29) (TriggeredSeconds :type Float%20%28double-precision%29) (InputAction :type Input%20Action%20Object%20Reference :default "/Game/Systems/GridSystem/DebugTools/DebugInputs/InputActions/GIA_Sideways.GIA_Sideways"))
  ;[1 1 1] Movement Logic
  (:Triggered
    (Variables|Default|SetLocation_Desired (+ (* (* ActionValue (Variables|Default|GetLocation_Speed)) (Transformation|GetActorRightVector)) (Variables|Default|GetLocation_Desired)))))

(event Input|EnhancedActionEvents|EnhancedInputActionGIA_RotateRight
  (params (ActionValue :type Boolean) (ElapsedSeconds :type Float%20%28double-precision%29) (TriggeredSeconds :type Float%20%28double-precision%29) (InputAction :type Input%20Action%20Object%20Reference :default "/Game/Systems/GridSystem/DebugTools/DebugInputs/InputActions/GIA_RotateRight.GIA_RotateRight"))
  ;[1 1 1] Rotate Camera
  (:Started
    (Variables|Default|SetRotation_Desired (Math|Rotator|CombineRotators (Variables|Default|GetRotation_Desired) (Math|Rotator|MakeRotator 0.0 0.0 (- 0.0 (Variables|Default|GetRotation_Speed)))))))

(event Input|EnhancedActionEvents|EnhancedInputActionGIA_RotateLeft
  (params (ActionValue :type Boolean) (ElapsedSeconds :type Float%20%28double-precision%29) (TriggeredSeconds :type Float%20%28double-precision%29) (InputAction :type Input%20Action%20Object%20Reference :default "/Game/Systems/GridSystem/DebugTools/DebugInputs/InputActions/GIA_RotateLeft.GIA_RotateLeft"))
  ;[1 1 1] Rotate Camera
  (:Started
    (Variables|Default|SetRotation_Desired (Math|Rotator|CombineRotators (Variables|Default|GetRotation_Desired) (Math|Rotator|MakeRotator 0.0 0.0 (Variables|Default|GetRotation_Speed))))))

(event EventTick
  (params (DeltaSeconds :type Float%20%28single-precision%29))
  (bind _cameraspring (Variables|Default|GetCameraSpring))
  (Variables|/Script/Engine.SpringArmComponent|SetTargetArmLength _cameraspring (Math|Interpolation|FInterpTo (Variables|/Script/Engine.SpringArmComponent|GetTargetArmLength _cameraspring) (Variables|Default|GetZoom_Desired) DeltaSeconds (Variables|Default|GetZoom_Interp)))
  (Transformation|SetActorLocation (Math|Interpolation|VInterpTo (Transformation|GetActorLocation) (Variables|Default|GetLocation_Desired) DeltaSeconds (Variables|Default|GetLocation_Interp)) false false)
  (Transformation|SetActorRotation (Math|Interpolation|RInterpTo (Transformation|GetActorRotation) (Variables|Default|GetRotation_Desired) DeltaSeconds (Variables|Default|GetRotation_Interp))))

(event EventBeginPlay
  (Variables|Default|SetLocation_Desired (Transformation|GetActorLocation))
  (Variables|Default|SetZoom_Desired (Variables|/Script/Engine.SpringArmComponent|GetTargetArmLength (Variables|Default|GetCameraSpring)))
  (Variables|Default|SetRotation_Desired (Transformation|GetActorRotation)))

(fn ConstructionScript)